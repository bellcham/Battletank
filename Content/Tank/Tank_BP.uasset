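; Tank Blueprint that sets up the vehicle's components and handles player input for camera, firing and driving.
; On BeginPlay it passes barrel and turret to TankAiming and both tracks to TankMovement.
; Look input rotates the azimuth gimbal and camera, while zoom sets clamped spring arm length and derives arm pitch from it.
; Driving supports direct per-track throttle or fly-by-wire intents through TankMovement; firing goes through TankAiming.
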(event `self.ReceiveBeginPlay`
  (`TankAimingComponent.Initialise` (`self.TankAiming`) (`self.TankBarrel`) (`self.TankTurret`))
  (`TankMovementComponent.Initialise` (`self.TankMovement`) (`self.LeftTrack`) (`self.RightTrack`)))

(event `InputAxis|AimAziumuth`
  (params (AxisValue :type "Float (single-precision)"))
  ;[1 1 1] Camera Input Binding
  (`SceneComponent.K2_AddLocalRotation` (`self.Azimuth Gimbal`) (`KismetMathLibrary.MakeRotator` 0.0 0.0 (* AxisValue (`GameplayStatics.GetWorldDeltaSeconds`) 100.0)) false false))

(event `InputAxis|AimElevation`
  (params (AxisValue :type "Float (single-precision)"))
  ;[1 1 1] Camera Input Binding
  (`SceneComponent.K2_AddLocalRotation` (`self.Camera`) (`KismetMathLibrary.MakeRotator` 0.0 (* AxisValue (`GameplayStatics.GetWorldDeltaSeconds`) 100.0)) false false))

(event `InputAxis|CameraZoom`
  (params (AxisValue :type "Float (single-precision)"))
  (bind _springarm (`self.SpringArm`))
  (bind (_relativerotation_roll _relativerotation_pitch _relativerotation_yaw) (`KismetMathLibrary.BreakRotator` (`SceneComponent.RelativeRotation` _springarm)))
  (bind _returnvalue (`KismetMathLibrary.FClamp` (+ (* AxisValue 500.0) (`SpringArmComponent.TargetArmLength` _springarm)) 1000.0 10000.0))
  ;[1 1 1] Camera Input Binding
  (set `SpringArmComponent.TargetArmLength` _returnvalue _springarm)
  (`SceneComponent.K2_SetRelativeRotation` _springarm (`KismetMathLibrary.MakeRotator` _relativerotation_roll (/ _returnvalue -200.0) _relativerotation_yaw) false false))

(event `InputAction|FireMainGun`
  (params (Key :type "Key Structure" :default "AnyKey"))
  ;[1 1 1] Firing Controls
  (:`Pressed`
    (`TankAimingComponent.Fire` (`self.TankAiming`))))

(event `InputAxis|LeftTrackThrottle`
  (params (AxisValue :type "Float (single-precision)"))
  (`TankTrack.SetThrottle` (`self.LeftTrack`) AxisValue))

(event `InputAxis|RightTrackThrottle`
  (params (AxisValue :type "Float (single-precision)"))
  (`TankTrack.SetThrottle` (`self.RightTrack`) AxisValue))

(event `InputAxis|FBW_Forward`
  (params (AxisValue :type "Float (single-precision)"))
  (`TankMovementComponent.IntendMoveForward` (`self.TankMovement`) AxisValue))

(event `InputAxis|FBW_Clockwise`
  (params (AxisValue :type "Float (single-precision)"))
  (`TankMovementComponent.IntendMoveClockwise` (`self.TankMovement`) AxisValue))

(fn `UserConstructionScript`)